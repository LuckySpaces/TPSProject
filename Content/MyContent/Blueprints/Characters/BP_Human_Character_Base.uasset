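; Base Blueprint for human characters that handles turn-in-place and aim state.
; BeginPlay caches the human AnimBP and starts a looping timer for the turn check.
; When aim yaw diverges far from actor yaw, a DoOnce-gated timeline lerps the actor toward it along the shortest path.
; Aim and NoAim set the AnimBP's aiming flag and toggle orient-rotation-to-movement.
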(event `self.ReceiveBeginPlay`
  ;[1 0.02535 0] BeginPlay Event
  ;;[0 0.1823 1] Set the play rate of the rotate character timeline
  (`TimelineComponent.SetPlayRate` (`self.Rotate Character`) 1.5)
  ;;[0 0.1823 1 1 15] Start the event timer for TurnInPlace
  (`KismetSystemLibrary.K2_SetTimerDelegate` (delegate `/Game/MyContent/Blueprints/Interfaces/BPI_Human_Character.TurnInPlace`) 0.1 true)
  ;;[0 0.1823 1] Get a reference to the human character animation blueprint
  (bind _asanim_bp_human_character (cast `/Game/MyContent/Blueprints/Animation_Bluprints/AnimBP_Human_Character` (`SkeletalMeshComponent.GetAnimInstance` (`self.Mesh`))))
  (set `self.AnimBPRef` _asanim_bp_human_character))

(event `/Game/MyContent/Blueprints/Interfaces/BPI_Human_Character.TurnInPlace`
  (bind _yaw (.yaw (`self.K2_GetActorRotation`)))
  (bind (_returnvalue_roll _returnvalue_pitch _returnvalue_yaw) (`KismetMathLibrary.BreakRotator` (`KismetMathLibrary.NormalizedDeltaRotator` (`self.K2_GetActorRotation`) (`self.GetBaseAimRotation`))))
  ;[1 0.01813 0] Turn in place event
  (if (> (`KismetMathLibrary.Abs` _returnvalue_yaw) 100.0)
    (`/Engine/EditorBlueprintResources/StandardMacros.DoOnce` false :!label _label
      (:`Completed`
        (set `self.GoToYRotation` (`KismetMathLibrary.ComposeRotators` (`KismetMathLibrary.MakeRotator` 0.0 0.0 _yaw) (`KismetMathLibrary.MakeRotator` 0.0 0.0 (- (.yaw (`self.GetBaseAimRotation`)) _yaw))))
        (bind (_direction _float_track) (`Timeline|Rotate Character` :!via `PlayFromStart`)
          (:`Update`
            (`self.K2_SetActorRotation` (`KismetMathLibrary.RLerp` (`self.K2_GetActorRotation`) (`self.GoToYRotation`) _float_track true)))
          (:`Finished`
            (goto _label :!via `Reset`)))))))

(event `/Game/MyContent/Blueprints/Interfaces/BPI_Human_Character.Aim`
  ;[1 0.02535 0] Aim Event
  (set `/Game/MyContent/Blueprints/Animation_Bluprints/AnimBP_Human_Character.IsAiming` true (`self.AnimBPRef`))
  (set `CharacterMovementComponent.bOrientRotationToMovement` false (`self.CharacterMovement`)))

(event `/Game/MyContent/Blueprints/Interfaces/BPI_Human_Character.NoAim`
  ;[1 0.02535 0] Aim Event
  (set `/Game/MyContent/Blueprints/Animation_Bluprints/AnimBP_Human_Character.IsAiming` false (`self.AnimBPRef`))
  (set `CharacterMovementComponent.bOrientRotationToMovement` true (`self.CharacterMovement`)))

(fn `UserConstructionScript`)