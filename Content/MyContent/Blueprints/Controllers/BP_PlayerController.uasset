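; BP_PlayerController is a player controller that routes movement, look and aim input to whichever pawn it controls.
; Move axes apply movement along control-yaw-only forward and right vectors, while turn and look-up axes feed controller yaw and pitch.
; Aim press and release send aim and field-of-view interface messages, only if the pawn implements both BPI_Human_Character and BPI_ControllableCharacter, checked through a helper function.
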(event `InputAxis|MoveForward`
  (params (AxisValue :type "Float (single-precision)"))
  (bind _returnvalue (`self.K2_GetPawn`))
  ;[1 0.02535 0] Movement
  (`Pawn.AddMovementInput` _returnvalue (`KismetMathLibrary.GetForwardVector` (`KismetMathLibrary.MakeRotator` 0.0 0.0 (.yaw (`Pawn.GetControlRotation` _returnvalue)))) AxisValue false))

(event `InputAxis|MoveRight`
  (params (AxisValue :type "Float (single-precision)"))
  (bind _returnvalue (`self.K2_GetPawn`))
  ;[1 0.02535 0] Movement
  (`Pawn.AddMovementInput` _returnvalue (`KismetMathLibrary.GetRightVector` (`KismetMathLibrary.MakeRotator` 0.0 0.0 (.yaw (`Pawn.GetControlRotation` _returnvalue)))) AxisValue false))

(event `InputAxis|Turn`
  (params (AxisValue :type "Float (single-precision)"))
  ;[1 0.02535 0] Look Around
  (`Pawn.AddControllerYawInput` (`self.K2_GetPawn`) AxisValue))

(event `InputAction|Aim`
  (params (Key :type "Key Structure"))
  (bind _returnvalue (`self.K2_GetPawn`))
  (bind _returnvalue_2 (and (`self.DoesControlledPawnHaveInterface` "/Game/MyContent/Blueprints/Interfaces/BPI_Human_Character.BPI_Human_Character_C") (`self.DoesControlledPawnHaveInterface` "/Game/MyContent/Blueprints/Interfaces/BPI_ControllableCharacter.BPI_ControllableCharacter_C")))
  ;[1 0.02535 0] Aim Input Event
  (:`Pressed`
    (if _returnvalue_2
      (message `/Game/MyContent/Blueprints/Interfaces/BPI_Human_Character.Aim` _returnvalue)
      (message `/Game/MyContent/Blueprints/Interfaces/BPI_ControllableCharacter.AimFieldOfViewPressed` _returnvalue)))
  (:`Released`
    (if _returnvalue_2
      (message `/Game/MyContent/Blueprints/Interfaces/BPI_Human_Character.NoAim` _returnvalue)
      (message `/Game/MyContent/Blueprints/Interfaces/BPI_ControllableCharacter.AimFieldOfViewReleased` _returnvalue))))

(event `InputAxis|LookUp`
  (params (AxisValue :type "Float (single-precision)"))
  ;[1 0.02535 0] Look Around
  (`Pawn.AddControllerPitchInput` (`self.K2_GetPawn`) AxisValue))

(fn `DoesControlledPawnHaveInterface`
  (params (Interface :type "Interface Class Reference"))
  (returns (ReturnValue :type Boolean))
  (return (`KismetSystemLibrary.DoesImplementInterface` (`self.K2_GetPawn`) Interface)))

(fn `UserConstructionScript`)