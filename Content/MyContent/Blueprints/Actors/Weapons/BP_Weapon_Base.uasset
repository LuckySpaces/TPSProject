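; Base weapon actor that handles single or automatic fire, clip and reserve ammo, and delayed reloading.
; StartShooting fires once and, for automatic weapons, loops FireBullet on a timer until StopShooting clears it.
; Each shot runs a debug-drawn muzzle line trace with no hit handling, plays the fire montage, and only notifies and spends ammo when the parent actor implements BPI_Human_Character.
; Reloading waits, then refills the clip from reserve.
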(event `/Game/MyContent/Blueprints/Interfaces/BPI_Weapon.StartShooting`
  ;[1 0.02535 0] StartShooting Event
  (if (`self.CanFire`)
    (set `self.IsFiring` true)
    (`self.FireBullet`)
    (if (`self.IsAutomatic`)
      (bind _returnvalue (`KismetSystemLibrary.K2_SetTimer` null "FireBullet" (`self.FireRate`) true))
      (set `self.GunTimer` _returnvalue))))

(event `/Game/MyContent/Blueprints/Interfaces/BPI_Weapon.StopShooting`
  (bind _guntimer (`self.GunTimer`))
  ;[1 0.02535 0] StopShooting Event
  (set `self.IsFiring` false)
  (if (`KismetSystemLibrary.K2_IsValidTimerHandle` _guntimer)
    (`KismetSystemLibrary.K2_ClearAndInvalidateTimerHandle` _guntimer)))

(event `/Game/MyContent/Blueprints/Interfaces/BPI_Weapon.Reloading`
  (params (Delay :type "Float (single-precision)"))
  ;[1 0.02535 0] Reloading Event
  (if (`self.CanReload`)
    (set `self.IsReloading` true)
    (`KismetSystemLibrary.Delay` Delay)
    (`self.ReloadBullets`)
    (set `self.IsReloading` false)))

(fn `BulletLineTrace`
  (bind _muzzle_location (`self.Muzzle_Location`))
  (bind _returnvalue (`SceneComponent.K2_GetComponentLocation` _muzzle_location))
  (`KismetSystemLibrary.LineTraceSingle` :`Start` _returnvalue :`End` (+ _returnvalue (* (`KismetMathLibrary.GetForwardVector` (`SceneComponent.K2_GetComponentRotation` _muzzle_location)) (`self.Range`))) :`TraceChannel` "TraceTypeQuery1" :`DrawDebugType` "ForDuration"))

(fn `CanFire`
  (returns (ReturnValue :type Boolean))
  (return (and (not (`self.IsReloading`)) (> (`self.AmmoCurrent`) 0))))

(fn `CanReload`
  (returns (ReturnValue :type Boolean))
  (return (and (not (`self.IsReloading`)) (< (`self.AmmoCurrent`) (`self.ClipSize`)))))

(fn `FireBullet`
  (bind _returnvalue (`self.GetParentActor`))
  (if (`self.CanFire`)
    (`self.BulletLineTrace`)
    (`AnimInstance.Montage_Play` (`SkeletalMeshComponent.GetAnimInstance` (`self.Gun`)) (`self.FireMontage`) 1.0 "MontageLength" 0.0 true)
    (if (`KismetSystemLibrary.DoesImplementInterface` _returnvalue "/Game/MyContent/Blueprints/Interfaces/BPI_Human_Character.BPI_Human_Character_C")
      (message `/Game/MyContent/Blueprints/Interfaces/BPI_Human_Character.Shoot` _returnvalue)
      (`/Engine/EditorBlueprintResources/StandardMacros.DecrementInt` (`self.AmmoCurrent`)))))

(fn `ReloadBullets`
  (locals (BulletDifference :type Integer))
  (bind _output_get (set `local.BulletDifference` (- (`self.ClipSize`) (`self.AmmoCurrent`))))
  (if (> (`self.AmmoMax`) _output_get)
    (set `self.AmmoCurrent` (`self.ClipSize`))
    (set `self.AmmoMax` (- (`self.AmmoMax`) (`local.BulletDifference`)))
    (else
      (set `self.AmmoCurrent` (+ (`self.AmmoCurrent`) (`self.AmmoMax`)))
      (set `self.AmmoMax` 0))))

(fn `UserConstructionScript`)